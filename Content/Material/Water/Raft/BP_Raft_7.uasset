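; Physics-driven raft that springs toward a target pose and lets that target travel with it while a Character is aboard.
; BeginPlay stores the start transform and creates a soft, lightly damped Physics Control and body modifier on the Cube mesh.
; While a Character overlaps the box, Tick retargets the control to the Cube's current XY, roll and yaw, retaining the starting height and pitch.
; On exit, the target stops updating.
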(event `self.ReceiveBeginPlay`
  (`self.PhysicsStart`))

(event `self.ReceiveTick`
  (params (DeltaSeconds :type "Float (single-precision)"))
  (`self.PhysicsMove`))

(event `self.BoxCollision.OnComponentBeginOverlap`
  (params (OverlappedComponent :type "PrimitiveComponent Object Reference") (OtherActor :type "Actor Object Reference") (OtherComp :type "PrimitiveComponent Object Reference") (OtherBodyIndex :type Integer) (bFromSweep :type Boolean) (SweepResult :type "HitResult Structure (by ref)"))
  (cast `Character` OtherActor)
  (set `self.Moving` true))

(event `PhysicsMove`
  (bind (_return_value_location_x _return_value_location_y _return_value_location_z) (`KismetMathLibrary.BreakVector` (`self.Return Value Location`)))
  (bind (_return_value_rotation_roll _return_value_rotation_pitch) (`KismetMathLibrary.BreakRotator` (`self.Return Value Rotation`)))
  (bind _returnvalue (`SceneComponent.K2_GetComponentToWorld` (`self.Cube`)))
  (if (`self.Moving`)
    (`PhysicsControlComponent.SetControlTargetPositionAndOrientation` (`self.PhysicsControl`) "test_0" (`KismetMathLibrary.MakeVector` (.x (.location _returnvalue)) (.y (.location _returnvalue)) _return_value_location_z) (`KismetMathLibrary.MakeRotator` (.roll (.rotation _returnvalue)) _return_value_rotation_pitch (.yaw (.rotation _returnvalue))) 0.0 true false)))

(event `self.BoxCollision.OnComponentEndOverlap`
  (params (OverlappedComponent :type "PrimitiveComponent Object Reference") (OtherActor :type "Actor Object Reference") (OtherComp :type "PrimitiveComponent Object Reference") (OtherBodyIndex :type Integer))
  (cast `Character` OtherActor)
  (set `self.Moving` false))

(fn `UserConstructionScript`)