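; BP_BrokenLight is a broken lamp in the day-night cycle scripts, with a point light and a Sparks effect.
; From BeginPlay, a self-calling Again event loops every two seconds, using a FlipFlop to alternate the sparks' User.Color parameter between orange and blue.
; A TurnOn/OffLights event sets the visibility of both the light and the sparks, while the color loop keeps running independently.
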(event `Again`
  (bind _sparks (`self.Sparks`))
  (`KismetSystemLibrary.Delay` 2.0 :!label _label)
  (`/Engine/EditorBlueprintResources/StandardMacros.FlipFlop`
    (:`A`
      (`FXSystemComponent.SetColorParameter` _sparks "User.Color" (struct :`R` 1.0 :`G` 0.254011 :`A` 1.0)))
    (:`B`
      (`FXSystemComponent.SetColorParameter` _sparks "User.Color" (struct :`G` 0.475386 :`B` 1.0 :`A` 1.0))))
  (`self.Again`))

(event `self.ReceiveBeginPlay`
  (goto _label))

(event `/Game/Scripts/DayNightCycle/Lamps/BP_IsLight.TurnOn/OffLights`
  (params (`TurnLightsOn?` :type Boolean))
  (`SceneComponent.SetVisibility` (`self.PointLight`) `TurnLightsOn?` false)
  (`SceneComponent.SetVisibility` (`self.Sparks`) `TurnLightsOn?` false))

(fn `UserConstructionScript`)